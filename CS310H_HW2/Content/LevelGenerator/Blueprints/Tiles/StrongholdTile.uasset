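; StrongholdTile is a level-generator tile Blueprint representing a stronghold that tracks health.
; Its TakeDamage function subtracts the given amount from Health and rewrites a text render component to show the new HP value.
; The function has no clamp or destruction check, and the event graph holds only disabled default events.
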(event EventBeginPlay
  (|CallParentFunction) ; This node is disabled and will not be called.\nDrag off pins to build functionality.
)

(event Collision|EventActorBeginOverlap
  (params (OtherActor :type Actor%20Object%20Reference))
  (|CallParentFunction OtherActor) ; This node is disabled and will not be called.\nDrag off pins to build functionality.
)

(event EventTick
  (params (DeltaSeconds :type Float%20%28single-precision%29))
  (|CallParentFunction DeltaSeconds) ; This node is disabled and will not be called.\nDrag off pins to build functionality.
)

(fn ConstructionScript
  (|CallParentFunction))

(fn TakeDamage
  (params (Amount :type Integer))
  (bind _output_get (Variables|Default|SetHealth (- (Variables|Default|GetHealth) Amount)))
  (Rendering|Components|TextRender|SetText (Variables|Default|GetHealthTextRender) (Utilities|Text|ToText(String) (Utilities|String|Append "HP: " (Utilities|String|ToString(Integer) _output_get)))))