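; Enemy spawn point actor for the level generator that spawns waves of randomly chosen enemy classes at an offset from its location.
; BeginPlay schedules Start Wave by timer, which resets the count and starts Spawn Enemy.
; Spawn Enemy re-arms its timer until the wave's quota is met, then schedules the next wave while any remain.
; Both functions print debug messages; randomized spawn spacing exists only in unconnected nodes.
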(event EventBeginPlay
  (Utilities|Time|SetTimerbyFunctionName 0 "Start Wave" (Variables|Default|GetTimeBetweenWaves)))

(event Collision|EventActorBeginOverlap
  (params (OtherActor :type Actor%20Object%20Reference))
  (|CallParentFunction OtherActor) ; This node is disabled and will not be called.\nDrag off pins to build functionality.
)

(event EventTick
  (params (DeltaSeconds :type Float%20%28single-precision%29))
  (|CallParentFunction DeltaSeconds) ; This node is disabled and will not be called.\nDrag off pins to build functionality.
)

(fn ConstructionScript
  (Variables|Default|SetSpawn%20Position (+ (Variables|Default|GetSpawn%20Offset) (.location (Transformation|GetActorTransform))))
  (Variables|Default|SetNumEnemyClasses (Utilities|Array|Length (Variables|Default|GetEnemies)))
  (|CallParentFunction))

(fn StartWave
  (Development|PrintString (Utilities|String|Append "Starting wave " (Utilities|String|ToString(Integer) (Variables|Default|GetCurrentWave))) true true "(R=0.000000,G=0.660000,B=1.000000,A=1.000000)" 1e+02)
  (Variables|Default|SetEnemiesSpawnedInWave 0)
  (Utilities|Time|SetTimerbyFunctionName 0 "Spawn Enemy" (Variables|Default|GetAverageTimeBetweenEnemies)))

(fn SpawnEnemy
  (bind _currentwave (Variables|Default|GetCurrentWave))
  (bind _enemiesperwave (Variables|Default|GetEnemiesPerWave))
  (bind _output (Utilities|Array|Get(acopy) _enemiesperwave _currentwave))
  (Development|PrintString (Utilities|String|Append (Utilities|String|Append (Utilities|String|Append "Spawning enemy " (Utilities|String|ToString(Integer) (Variables|Default|GetEnemiesSpawnedInWave))) " out of ") (Utilities|String|ToString(Integer) _output)) true true "(R=0.000000,G=0.660000,B=1.000000,A=1.000000)" 1e+01)
  (Game|SpawnActorfromClass (Utilities|Array|Get(acopy) (Variables|Default|GetEnemies) (Math|Random|RandomInteger (Variables|Default|GetNumEnemyClasses))) (Math|Transform|MakeTransform (Variables|Default|GetSpawn%20Position) "0, 0, 0" "1.000000,1.000000,1.000000") "Undefined" 0 0)
  (bind _result (Math|Integer|IncrementInt (Variables|Default|GetEnemiesSpawnedInWave))
    (:%20%20
      (if (== _result _output)
        (bind _result_2 (Math|Integer|IncrementInt (Variables|Default|GetCurrentWave))
          (:%20%20
            (if (< _result_2 (Variables|Default|GetNumWaves))
              (Utilities|Time|SetTimerbyFunctionName 0 "Start Wave" (Variables|Default|GetTimeBetweenWaves)))))
        (else
          (Utilities|Time|SetTimerbyFunctionName 0 "Spawn Enemy" (Variables|Default|GetAverageTimeBetweenEnemies)))))))