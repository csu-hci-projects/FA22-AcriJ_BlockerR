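; World generator actor that builds a tile grid with a randomly winding path across it on BeginPlay.
; InitializeTiles fills parallel tile-coordinate and tile-type arrays with grass.
; BuildPath walks the columns from a random starting row, randomly inserting one-row left or right jogs as paired turn tiles, finding indices by linear search.
; SpawnTiles then spawns the matching tile actor for each entry, scaled and offset from the generator's location.
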(event EventBeginPlay
  (CallFunction|InitializeTiles)
  (CallFunction|BuildPath)
  (CallFunction|SpawnTiles))

(fn ConstructionScript)

(fn InitializeTiles
  (for _index (range 0 (- (Variables|Default|GetNumCols) 1))
    (for _index_2 (range 0 (- (Variables|Default|GetNumRows) 1))
      (bind _returnvalue (Utilities|Array|Add (Variables|Default|GetTiles) (Utilities|Struct|MakeTile _index _index_2)))
      (Utilities|Array|Insert (Variables|Default|GetTile%20Types) "NewEnumerator0" _returnvalue))))

(fn SpawnTiles
  (bind _self self)
  (for _array_element (Variables|Default|GetTiles)
    (switch Utilities|FlowControl|Switch|SwitchonTileType (Utilities|Array|Get(acopy) (Variables|Default|GetTile%20Types) (Utilities|Array|FindItem (Variables|Default|GetTiles) _array_element))
      (:NewEnumerator0
        (Game|SpawnActorfromClass "/Game/LevelGenerator/Blueprints/Tiles/GrassTile.GrassTile_C" (Math|Transform|MakeTransform (+ (* (Math|Vector|MakeVector (Math|Conversions|ToFloat(Integer) (.X (Utilities|Struct|BreakTile _array_element))) (Math|Conversions|ToFloat(Integer) (.Y (Utilities|Struct|BreakTile _array_element))) 0.0) (Variables|Default|GetTileScale)) (Transformation|GetActorLocation)) "0, 0, 0" "1.000000,1.000000,1.000000") "Undefined" 0 (.X (Utilities|Struct|BreakTile _array_element)) (.Y (Utilities|Struct|BreakTile _array_element)) _self 0))
      (:NewEnumerator1
        (Game|SpawnActorfromClass "/Game/LevelGenerator/Blueprints/Tiles/StraightPathTile.StraightPathTile_C" (Math|Transform|MakeTransform (+ (* (Math|Vector|MakeVector (Math|Conversions|ToFloat(Integer) (.X (Utilities|Struct|BreakTile _array_element))) (Math|Conversions|ToFloat(Integer) (.Y (Utilities|Struct|BreakTile _array_element))) 0.0) (Variables|Default|GetTileScale)) (Transformation|GetActorLocation)) "0, 0, 0" "1.000000,1.000000,1.000000") "Undefined" 0 (.X (Utilities|Struct|BreakTile _array_element)) (.Y (Utilities|Struct|BreakTile _array_element)) _self 0))
      (:NewEnumerator2
        (Game|SpawnActorfromClass "/Game/LevelGenerator/Blueprints/Tiles/ForwardRightTurnPath.ForwardRightTurnPath_C" (Math|Transform|MakeTransform (+ (* (Math|Vector|MakeVector (Math|Conversions|ToFloat(Integer) (.X (Utilities|Struct|BreakTile _array_element))) (Math|Conversions|ToFloat(Integer) (.Y (Utilities|Struct|BreakTile _array_element))) 0.0) (Variables|Default|GetTileScale)) (Transformation|GetActorLocation)) "0, 0, 0" "1.000000,1.000000,1.000000") "Undefined" 0 (.X (Utilities|Struct|BreakTile _array_element)) (.Y (Utilities|Struct|BreakTile _array_element)) _self 0))
      (:NewEnumerator3
        (Game|SpawnActorfromClass "/Game/LevelGenerator/Blueprints/Tiles/ForwardLeftTurnPath.ForwardLeftTurnPath_C" (Math|Transform|MakeTransform (+ (* (Math|Vector|MakeVector (Math|Conversions|ToFloat(Integer) (.X (Utilities|Struct|BreakTile _array_element))) (Math|Conversions|ToFloat(Integer) (.Y (Utilities|Struct|BreakTile _array_element))) 0.0) (Variables|Default|GetTileScale)) (Transformation|GetActorLocation)) "0, 0, 0" "1.000000,1.000000,1.000000") "Undefined" 0 (.X (Utilities|Struct|BreakTile _array_element)) (.Y (Utilities|Struct|BreakTile _array_element)) _self 0))
      (:NewEnumerator4
        (Game|SpawnActorfromClass "/Game/LevelGenerator/Blueprints/Tiles/BackwardRightTurnPath.BackwardRightTurnPath_C" (Math|Transform|MakeTransform (+ (* (Math|Vector|MakeVector (Math|Conversions|ToFloat(Integer) (.X (Utilities|Struct|BreakTile _array_element))) (Math|Conversions|ToFloat(Integer) (.Y (Utilities|Struct|BreakTile _array_element))) 0.0) (Variables|Default|GetTileScale)) (Transformation|GetActorLocation)) "0, 0, 0" "1.000000,1.000000,1.000000") "Undefined" 0 (.X (Utilities|Struct|BreakTile _array_element)) (.Y (Utilities|Struct|BreakTile _array_element)) 0 0))
      (:NewEnumerator5
        (Game|SpawnActorfromClass "/Game/LevelGenerator/Blueprints/Tiles/BackwardLeftTurnPath.BackwardLeftTurnPath_C" (Math|Transform|MakeTransform (+ (* (Math|Vector|MakeVector (Math|Conversions|ToFloat(Integer) (.X (Utilities|Struct|BreakTile _array_element))) (Math|Conversions|ToFloat(Integer) (.Y (Utilities|Struct|BreakTile _array_element))) 0.0) (Variables|Default|GetTileScale)) (Transformation|GetActorLocation)) "0, 0, 0" "1.000000,1.000000,1.000000") "Undefined" 0 (.X (Utilities|Struct|BreakTile _array_element)) (.Y (Utilities|Struct|BreakTile _array_element)) _self 0)))))

(fn BuildPath
  (LocalVariables|SetCurrentRow (Math|Random|RandomInteger (Variables|Default|GetNumRows)))
  (while (< (LocalVariables|GetCurrentCol) (Variables|Default|GetNumCols))
    (bind _tileindex (CallFunction|GetTile (LocalVariables|GetCurrentCol) (LocalVariables|GetCurrentRow)))
    (CallFunction|MakeTilePath _tileindex "NewEnumerator1")
    (Math|Integer|IncrementInt (LocalVariables|GetCurrentCol)
      (:%20%20
        (if (Math|Random|RandomBool)
          (if (Math|Random|RandomBool)
            (if (and (< (LocalVariables|GetCurrentCol) (- (Variables|Default|GetNumCols) 1)) (< (LocalVariables|GetCurrentRow) (Variables|Default|GetNumRows)))
              (bind _tileindex_2 (CallFunction|GetTile (LocalVariables|GetCurrentCol) (LocalVariables|GetCurrentRow)))
              (CallFunction|MakeTilePath _tileindex_2 "NewEnumerator2")
              (Math|Integer|IncrementInt (LocalVariables|GetCurrentRow)
                (:%20%20
                  (bind _tileindex_3 (CallFunction|GetTile (LocalVariables|GetCurrentCol) (LocalVariables|GetCurrentRow)))
                  (CallFunction|MakeTilePath _tileindex_3 "NewEnumerator4")
                  (Math|Integer|IncrementInt (LocalVariables|GetCurrentCol) :!label _label))))
            (elif (and (< (LocalVariables|GetCurrentCol) (- (Variables|Default|GetNumCols) 1)) (> (LocalVariables|GetCurrentRow) 0))
              (bind _tileindex_4 (CallFunction|GetTile (LocalVariables|GetCurrentCol) (LocalVariables|GetCurrentRow)))
              (CallFunction|MakeTilePath _tileindex_4 "NewEnumerator3")
              (Math|Integer|DecrementInt (LocalVariables|GetCurrentRow)
                (:%20%20
                  (bind _tileindex_5 (CallFunction|GetTile (LocalVariables|GetCurrentCol) (LocalVariables|GetCurrentRow)))
                  (CallFunction|MakeTilePath _tileindex_5 "NewEnumerator5")
                  (goto _label))))))))))

(fn MakeTilePath
  (params (TileIndex :type Integer) (Tile%20Type :type TileType%20Enum :default "NewEnumerator0"))
  (|SetBy-RefVar (Utilities|Array|Get(acopy) (Variables|Default|GetTile%20Types) TileIndex) Tile%20Type)
  (return))

(fn GetTile
  (params (X :type Integer) (Y :type Integer))
  (for (_array_element _array_index) (Variables|Default|GetTiles)
    (if (and (== (.x _array_element) X) (== (.y _array_element) Y))
      (return _array_index))))